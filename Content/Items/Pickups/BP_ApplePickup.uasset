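; BP_ApplePickup is an apple pickup whose event graph holds only disconnected fragments, so none of its logic runs.
; The fragments cast to BP_Player, add apples up to MaxApples, save the count to the player's SaveGame slot, and destroy the actor.
; No event triggers these fragments, and the construction script is empty.
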(fn `UserConstructionScript`)