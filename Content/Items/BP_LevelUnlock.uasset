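; BP_LevelUnlock is a trigger actor that unlocks a level and sends the player there.
; When BP_Player overlaps its Box, it sets the LevelNumber entry in the player's SaveGame Levels array to true and saves to a fixed slot.
; It then shows a WBP_Fade widget and, after a short delay, opens the Level referenced by its variable.
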(event `self.Box.OnComponentBeginOverlap`
  (params (OverlappedComponent :type "PrimitiveComponent Object Reference") (OtherActor :type "Actor Object Reference") (OtherComp :type "PrimitiveComponent Object Reference") (OtherBodyIndex :type Integer) (bFromSweep :type Boolean) (SweepResult :type "HitResult Structure (by ref)"))
  (bind _asbp_player (cast `/Game/PlayerCharacter/BP_Player` OtherActor))
  (bind _save_game (`/Game/PlayerCharacter/BP_Player.Save Game` _asbp_player))
  (`KismetArrayLibrary.Array_Set` (`/Game/GameFeatures/BP_SaveGame.Levels` _save_game) (`self.Level Number`) true)
  (`GameplayStatics.SaveGameToSlot` _save_game "1")
  (bind _returnvalue (`|CreateWidget` "/Game/UI/InGame/WBP_Fade.WBP_Fade_C"))
  (`UserWidget.AddToViewport` _returnvalue 0)
  (`KismetSystemLibrary.Delay` 1.0)
  (`GameplayStatics.OpenLevelBySoftObjectPtr` (`self.Level`)))

(fn `UserConstructionScript`)