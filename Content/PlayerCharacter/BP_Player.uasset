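; BP_Player is the player character Blueprint, handling box damage, pause input and air-dash reset.
; DamageBox forwards to the passed BP_Box, and landing sets DashInAir back to one.
; The pause input creates a WBP_PauseMenu widget and adds it to the viewport.
; BeginPlay is empty, and logic loading Apples, Lives and Coins from BP_SaveGame is disconnected, so it never runs.
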(event `self.DamageBox`
  (params (Box :type "Actor Object Reference"))
  (bind _asbp_box (cast `/Game/Items/Box/BP_Box` Box))
  (`/Game/Items/Box/BP_Box.DamageBox` _asbp_box))

(event `self.OnLanded`
  (params (Hit :type "HitResult Structure (by ref)"))
  ;[1 1 1] Reset Dash In Air
  (set `self.DashInAir` 1.0))

(event `self.ReceiveBeginPlay`
  ;[1 1 1] Begin Play
)

(event `EnhancedInput|/Game/Input/Action/IA_Pause`
  (params (ActionValue :type Boolean) (ElapsedSeconds :type "Float (double-precision)") (TriggeredSeconds :type "Float (double-precision)") (InputAction :type "InputAction Object Reference" :default "/Game/Input/Action/IA_Pause.IA_Pause"))
  ;[1 1 1] Pause
  (:`Started`
    (bind _returnvalue (`|CreateWidget` "/Game/UI/InGame/WBP_PauseMenu.WBP_PauseMenu_C"))
    (`UserWidget.AddToViewport` _returnvalue 0)))

(fn `UserConstructionScript`)